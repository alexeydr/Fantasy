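; BP_RewardViking is a reward item Blueprint that grants the player a max health bonus while equipped.
; Its EquipedEffect event casts the player character to MainCharacter and adds a fixed amount to MaxHealth on its StatsComp.
; UnEquipedEffect subtracts the same amount, and both events change only max health, leaving current health untouched.
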(event EventBeginPlay
  (|CallParentFunction) ; This node is disabled and will not be called.\nDrag off pins to build functionality.
)

(event Collision|EventActorBeginOverlap
  (params (OtherActor :type Actor%20Object%20Reference))
  (|CallParentFunction OtherActor) ; This node is disabled and will not be called.\nDrag off pins to build functionality.
)

(event EventTick
  (params (DeltaSeconds :type Float%20%28single-precision%29))
  (|CallParentFunction DeltaSeconds) ; This node is disabled and will not be called.\nDrag off pins to build functionality.
)

(event EventEquipedEffect
  (bind _asmain_character (Utilities|Casting|CastToMainCharacter (Game|GetPlayerCharacter 0)))
  (Variables|/Script/Fantasy.StatsComponent|SetMaxHealth (Variables|/Script/Fantasy.MainCharacter|GetStatsComp _asmain_character) (+ (Variables|/Script/Fantasy.StatsComponent|GetMaxHealth (Variables|/Script/Fantasy.MainCharacter|GetStatsComp _asmain_character)) 1e+02)))

(event EventUnEquipedEffect
  (bind _asmain_character (Utilities|Casting|CastToMainCharacter (Game|GetPlayerCharacter 0)))
  (Variables|/Script/Fantasy.StatsComponent|SetMaxHealth (Variables|/Script/Fantasy.MainCharacter|GetStatsComp _asmain_character) (- (Variables|/Script/Fantasy.StatsComponent|GetMaxHealth (Variables|/Script/Fantasy.MainCharacter|GetStatsComp _asmain_character)) 1e+02)))

(fn ConstructionScript
  (|CallParentFunction))