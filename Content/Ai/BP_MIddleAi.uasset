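; BP_MIddleAi is an AI Blueprint with a randomized task list and a random skeletal mesh.
; When NeedRandom is set, the construction script calls Random, which shuffles AllAvailableTasksDT row names, looks each up in MiddleTasks and stores found names in SelectedTasks.
; Random then puts a random Heads mesh on SKBowknot.
; BeginPlay repositions the widget component and re-rolls only that mesh, leaving the tasks untouched.
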(event Custom|Random
  (Utilities|FlowControl|Sequence
    (:then_0
      (Utilities|Array|Clear (Variables|Default|GetSelectedTasks))
      (bind _outrownames (DataTable|GetDataTableRowNames (Variables|Default|GetAllAvailableTasksDT)))
      (Utilities|Array|Shuffle _outrownames)
      (for _array_element _outrownames
        (bind _returnvalue (Utilities|GetDataTableRow "/Game/Ai/BotTasks/MiddleTasks/MiddleTasks.MiddleTasks" _array_element)
          (:then
            (Utilities|Array|Add (Variables|Default|GetSelectedTasks) (.Name (Utilities|Struct|BreakBotTask _returnvalue)))))))
    (:then_1
      (Class|SkinnedMeshComponent|SetSkeletalMesh (Variables|Default|GetSK_Bow-knot) (.OutItem (Utilities|Array|Random (Variables|Default|GetHeads))) false))))

(event EventBeginPlay
  (Transformation|SetRelativeLocation (Variables|Default|GetWidgetComp) "0,-40.000000,100.000000" false false)
  (Class|SkinnedMeshComponent|SetSkeletalMesh (Variables|Default|GetSK_Bow-knot) (.OutItem (Utilities|Array|Random (Variables|Default|GetHeads))) false))

(fn ConstructionScript
  (if (Variables|Default|GetbNeedRandom)
    (CallFunction|Random)))