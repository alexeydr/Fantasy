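; BP_MageAi is a mage enemy AI character that controls how it turns relative to the player.
; Each tick, RotationToChar enables orient-rotation-to-movement only when the player is farther than the attack distance plus a small margin.
; Unless fight mode is active and the player is beyond that range, it smoothly interpolates the actor's rotation to face the player.
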(event EventTick
  (params (DeltaSeconds :type Float%20%28single-precision%29))
  (CallFunction|RotationtoChar DeltaSeconds))

(fn ConstructionScript)

(fn RotationtoChar
  (params (DeltaTime :type Float%20%28single-precision%29))
  (bind _returnvalue (Game|GetPlayerCharacter 0))
  (bind _output_get (Variables|/Script/Engine.CharacterMovementComponent|SetbOrientRotationToMovement (Variables|Character|GetCharacterMovement) (> (Transformation|GetDistanceTo _returnvalue self) (+ (Variables|Default|GetAttackDistance) 1e+02))))
  (if (not (and (Variables|Default|GetbFightModeActive) _output_get))
    (bind _output_get_2 (LocalVariables|SetTargetRot (Math|Rotator|FindLookatRotation (Transformation|GetActorLocation) (Transformation|GetActorLocation _returnvalue))))
    (Transformation|SetActorRotation (Math|Interpolation|RInterpTo (Transformation|GetActorRotation) _output_get_2 DeltaTime 2e+01))))