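; BP_MagicanLeader is an interactable magician leader that opens a shop selling spells.
; On interaction it rebuilds its assortment by wrapping each entry of SpellsForSale in a new SalableSpell object and converting it with MakeSalebleItems.
; A newly created BP_ShopWidget receives that assortment and is added to the viewport.
; On BeginPlay it also repositions its widget component.
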(event EventBeginPlay
  (Transformation|SetRelativeLocation (Variables|Default|GetWidgetComp) "0,-40.000000,100.000000" false false))

(event EventOnInteraction
  (Utilities|Array|Clear (Variables|Default|GetAssortment))
  (bind _returnvalue (UserInterface|CreateWidget "/Game/UI/Shop/BP_ShopWidget.BP_ShopWidget_C"))
  (Variables|Default|SetShopWidget _returnvalue)
  (for _array_element (Variables|Default|GetSpellsForSale)
    (bind _returnvalue_2 (Game|ConstructObjectfromClass "/Script/Fantasy.SalableSpell" self))
    (Variables|/Script/Fantasy.SalableSpell|SetSpellForSale _returnvalue_2 _array_element)
    (Utilities|Array|Add (Variables|Default|GetAssortment) (Utilities|Struct|MakeSalebleItems _returnvalue_2)))
  (Class|ShopUserWidget|CreateAssortment (Variables|Default|GetShopWidget) (Variables|Default|GetAssortment))
  (UserInterface|Viewport|AddtoViewport (Variables|Default|GetShopWidget) 0))

(fn ConstructionScript)